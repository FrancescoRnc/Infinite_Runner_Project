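; Player character for an infinite runner that shifts between three lanes and ends the game on a fatal hit.
; BeginPlay caches lane points around the spawn position; held left/right inputs call MoveHorizontal toward a side, and release returns to center.
; Lock/Unlock events pop and push these bindings on the controller's multi-input components.
; Overlaps decrement HealthComponent; when that returns true, input locks, collision and mesh turn off, and the GameMode's GameOver runs.
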(event `self.ReceiveBeginPlay`
  (bind _returnvalue (`self.K2_GetActorLocation`))
  (bind _returnvalue_2 (`self.GetActorRightVector`))
  (set `self.Points` (`|MakeArray` (+ (* _returnvalue_2 -300.0) _returnvalue) _returnvalue (+ (* _returnvalue_2 300.0) _returnvalue))))

(event `self.ReceiveActorBeginOverlap`
  (params (OtherActor :type "Actor Object Reference"))
  (bind _returnvalue (`HealthComponent.Decrease` (`self.HealthComponent`) 1))
  (if _returnvalue
    (`self.Lock Movement`)
    (`PrimitiveComponent.SetCollisionEnabled` (`self.CapsuleComponent`) "NoCollision")
    (`SceneComponent.SetVisibility` (`self.Mesh`) false false)
    (`InfiniteRunnerGameGameModeBase.GameOver` (cast `/Game/Gameplay/Mechanics/BP_InfiniteRunnerGM` (`GameplayStatics.GetGameMode`) :!pure true))))

(event `Unlock Movement`
  (bind _multiinputcomponent_release (`/Game/Gameplay/Mechanics/BP_InfiniteRunnerPC.MultiInputComponent_Release` (cast `/Game/Gameplay/Mechanics/BP_InfiniteRunnerPC` (`GameplayStatics.GetPlayerController` 0) :!pure true)))
  (bind _multiinputcomponent_press (`/Game/Gameplay/Mechanics/BP_InfiniteRunnerPC.MultiInputComponent_Press` (cast `/Game/Gameplay/Mechanics/BP_InfiniteRunnerPC` (`GameplayStatics.GetPlayerController` 0) :!pure true)))
  ;[1 1 1] Unlock Movement Input
  (`|ExecutionSequence`
    (:`then_0`
      (`MultiInputControlComponent.PushNewFunction` _multiinputcomponent_press "PadRight" (delegate `Move Right`)))
    (:`then_1`
      (`MultiInputControlComponent.PushNewFunction` _multiinputcomponent_press "PadLeft" (delegate `Move Left`)))
    (:`then_2`
      (`MultiInputControlComponent.PushNewFunction` _multiinputcomponent_release "PadRight" (delegate `Move Center`)))
    (:`then_3`
      (`MultiInputControlComponent.PushNewFunction` _multiinputcomponent_release "PadLeft" (delegate `Move Center`)))))

(event `Lock Movement`
  (bind _multiinputcomponent_press (`/Game/Gameplay/Mechanics/BP_InfiniteRunnerPC.MultiInputComponent_Press` (cast `/Game/Gameplay/Mechanics/BP_InfiniteRunnerPC` (`GameplayStatics.GetPlayerController` 0) :!pure true)))
  (bind _multiinputcomponent_release (`/Game/Gameplay/Mechanics/BP_InfiniteRunnerPC.MultiInputComponent_Release` (cast `/Game/Gameplay/Mechanics/BP_InfiniteRunnerPC` (`GameplayStatics.GetPlayerController` 0) :!pure true)))
  ;[1 1 1] Lock Movement Input
  (`|ExecutionSequence`
    (:`then_0`
      (`MultiInputControlComponent.PopLastFunction` _multiinputcomponent_press "PadRight"))
    (:`then_1`
      (`MultiInputControlComponent.PopLastFunction` _multiinputcomponent_press "PadLeft"))
    (:`then_2`
      (`MultiInputControlComponent.PopLastFunction` _multiinputcomponent_release "PadRight"))
    (:`then_3`
      (`MultiInputControlComponent.PopLastFunction` _multiinputcomponent_release "PadLeft"))))

(event `Move Right`
  ;[1 1 1] Unlock Movement Input
  (`InputMovable.MoveHorizontal` (`|GetArrayItem` (`self.Points`) 2)))

(event `Move Left`
  ;[1 1 1] Unlock Movement Input
  (`InputMovable.MoveHorizontal` (`|GetArrayItem` (`self.Points`))))

(event `Move Center`
  ;[1 1 1] Unlock Movement Input
  (`InputMovable.MoveHorizontal` (`|GetArrayItem` (`self.Points`) 1)))

(fn `UserConstructionScript`)