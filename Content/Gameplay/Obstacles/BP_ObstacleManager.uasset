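; BP_ObstacleManager is an obstacle manager that prepares a pool of wall obstacles and places them in the level.
; On BeginPlay it creates a stock of BP_ObstacleWall instances, stores it as MainStock and prints its size for debugging.
; After a short delay it passes the stock to LocateObstacles with a disposition index to position the walls.
; An unconnected branch would extract items from the stock into ActiveItems but never runs.
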(event `self.ReceiveBeginPlay`
  (bind _returnvalue (`ObstacleCreator.CreateStock` "/Game/Gameplay/Obstacles/BP_ObstacleWall.BP_ObstacleWall_C" 15))
  ;[1 1 1] Debug delle quantita'
  (bind _output_get (set `self.MainStock` _returnvalue))
  (`KismetSystemLibrary.PrintString` (`KismetStringLibrary.Concat_StrStr` "Stock Length: " (`KismetStringLibrary.Conv_IntToString` (`KismetArrayLibrary.Array_Length` _output_get))))
  (`KismetSystemLibrary.PrintString` "GO!")
  (`KismetSystemLibrary.Delay` 3.0)
  (`KismetSystemLibrary.PrintString` "Locate")
  (`ObstacleLocator.LocateObstacles` _output_get))

(fn `UserConstructionScript`)